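; BP_Aura_MainMenu is the main menu scene actor, which shows the menu UI and animates decorative props.
; On BeginPlay it caches the fireball's location, creates WBP_MainMenu and switches the player to UI-only input with a visible cursor.
; Each Tick advances a timer that resets past a full sine period, bobs the fireball vertically by that sine times an amplitude, and spins the magic circle around its local roll axis.
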(event `self.ReceiveBeginPlay`
  (bind _returnvalue (`GameplayStatics.GetPlayerController` 0))
  (set `self.FireballInitalLocaiton` (`SceneComponent.K2_GetComponentLocation` (`self.FireBall`)))
  (`/Engine/EditorBlueprintResources/StandardMacros.IsValid` (`GameplayStatics.GetPlayerController` 0)
    (:`Is Valid`
      (bind _returnvalue_2 (`|CreateWidget` "/Game/Blueprints/UI/MainMenu/WBP_MainMenu.WBP_MainMenu_C"))
      (`UserWidget.AddToViewport` _returnvalue_2 0)
      (`WidgetBlueprintLibrary.SetInputMode_UIOnlyEx` _returnvalue _returnvalue_2)
      (set `PlayerController.bShowMouseCursor` true _returnvalue))))

(event `self.ReceiveTick`
  (params (DeltaSeconds :type "Float (single-precision)"))
  (`self.UpdateTime` DeltaSeconds)
  (`SceneComponent.K2_SetWorldLocation` (`self.FireBall`) (+ (`self.FireballInitalLocaiton`) (`KismetMathLibrary.MakeVector` 0.0 0.0 (`self.SinTime`))) false false)
  (`SceneComponent.K2_AddLocalRotation` (`self.MagicCircle`) (`KismetMathLibrary.MakeRotator` (* (`GameplayStatics.GetWorldDeltaSeconds`) (`self.MagicCIrcleRotationRate`))) false false))

(fn `SinTime`
  (returns (ReturnValue :type "Float (double-precision)"))
  (return (* (`KismetMathLibrary.Sin` (`self.Time`)) (`self.Amplitude`))))

(fn `UpdateTime`
  (params (Time :type "Float (double-precision)"))
  (bind _output_get (set `self.Time` (+ Time (`self.Time`))))
  (if (> _output_get 6.28318)
    (set `self.Time` 0.0)))

(fn `UserConstructionScript`)