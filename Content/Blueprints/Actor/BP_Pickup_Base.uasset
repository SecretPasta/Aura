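; Base pickup actor that animates its spawn with sound, then hovers and spins until it is destroyed.
; On BeginPlay, a timeline drives scale and a height offset from the initial location, firing a one-shot ground impact sound past an elevation threshold.
; When the timeline finishes, it starts sinusoidal movement and rotation, defined outside these graphs.
; Tick applies the calculated location and rotation, and destruction plays the consumed sound.
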(event `self.ReceiveBeginPlay`
  (bind _scale (`self.Scale`))
  (`GameplayStatics.PlaySoundAtLocation` (`self.SpawnSound`) (`self.K2_GetActorLocation`) (struct) 1.0 1.0 0.0 null null null null)
  (bind (_direction _elevation _scale_2) (`Timeline|PickupElevationTimeline`)
    (:`Update`
      (set `self.Elevation` _elevation)
      (set `self.Scale` _scale_2)
      (set `self.CalculatedLocation` (`self.CalculateElevation` (`self.Elevation`)))
      (`self.SetActorScale3D` (`KismetMathLibrary.MakeVector` _scale _scale _scale))
      (if (> (`self.Elevation`) 0.8)
        (`/Engine/EditorBlueprintResources/StandardMacros.DoOnce` false
          (:`Completed`
            (`GameplayStatics.PlaySoundAtLocation` (`self.GroundImpactSound`) (`self.K2_GetActorLocation`) (struct) 1.0 1.0 0.0 null null null null)))))
    (:`Finished`
      (`self.StartSinusoidalMovement`)
      (`self.StartRotation`))))

(event `self.ReceiveTick`
  (params (DeltaSeconds :type "Float (single-precision)"))
  (`self.K2_SetActorLocation` (`self.CalculatedLocation`))
  (`self.K2_SetActorRotation` (`self.CalculatedRotation`)))

(event `self.ReceiveDestroyed`
  (`GameplayStatics.PlaySoundAtLocation` (`self.ConsumedSound`) (`self.K2_GetActorLocation`) (struct) 1.0 1.0 0.0 null null null null))

(fn `CalculateElevation`
  (params (A :type "Float (double-precision)"))
  (returns (ReturnValue :type "Vector Structure"))
  (bind (_initiallocation_x _initiallocation_y _initiallocation_z) (`KismetMathLibrary.BreakVector` (`self.InitialLocation`)))
  (return (`KismetMathLibrary.MakeVector` _initiallocation_x _initiallocation_y (+ _initiallocation_z (* A (`self.SpawnApex`))))))

(fn `UserConstructionScript`)